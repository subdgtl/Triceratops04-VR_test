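; VR motion controller actor that grabs and drops nearby actors and finds a teleport destination, with its hand set by EHand at construction.
; While teleporting is active, Tick line-traces forward from the controller and stores blocking hit locations, without moving the player.
; Grab and release send pickup and drop messages to the actor, which handles attachment itself.
; Pickup always reports the Left hand, whatever EHand is.
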(event `self.ReceiveTick`
  (params (DeltaSeconds :type "Float (single-precision)"))
  (bind (_bblockinghit _binitialoverlap _time _distance _location) (`GameplayStatics.BreakHitResult` (`self.LineTraceForward`)))
  (if (`self.bShouldTrace`)
    (bind _output_get (set `self.bTraceSuccess` _bblockinghit))
    (if _output_get
      (set `self.TeleportDestination` _location))))

(fn `ActivateTeleporter`
  (set `self.bShouldTrace` true))

(fn `DisableTeleporter`
  (set `self.bShouldTrace` false))

(fn `GrabActor`
  (returns (Success :type Boolean))
  (bind _nearestactor (`/Game/Blueprints/Pickup/BPL_PickTools.GetActorNearComponent` (`self.Hand`)))
  (`/Engine/EditorBlueprintResources/StandardMacros.IsValid` _nearestactor
    (:`Is Valid`
      (`|ExecutionSequence`
        (:`then_0`
          (set `self.AttachedActor` _nearestactor))
        (:`then_1`
          (message `/Game/Blueprints/Pickup/BPI_Pickable.Pickup` _nearestactor (`self.MotionController`) "Left"))
        (:`then_2`
          (return true))))
    (:`Is Not Valid`
      (return false))))

(fn `LineTraceForward`
  (returns (OutHit :type "HitResult Structure"))
  (bind _motioncontroller (`self.MotionController`))
  (bind _returnvalue (`SceneComponent.K2_GetComponentLocation` _motioncontroller))
  (bind _outhit (`KismetSystemLibrary.LineTraceSingle` :`Start` _returnvalue :`End` (+ _returnvalue (* (`KismetMathLibrary.GetForwardVector` (`SceneComponent.K2_GetComponentRotation` _motioncontroller)) 2500.0)) :`TraceChannel` "TraceTypeQuery1" :`DrawDebugType` "ForOneFrame"))
  (return _outhit))

(fn `ReleaseActor`
  (returns (Success :type Boolean))
  (bind _attachedactor (`self.AttachedActor`))
  (`/Engine/EditorBlueprintResources/StandardMacros.IsValid` _attachedactor
    (:`Is Valid`
      (message `/Game/Blueprints/Pickup/BPI_Pickable.Drop` _attachedactor (`self.MotionController`))
      (`|ExecutionSequence`
        (:`then_0`
          (set `self.AttachedActor` null))
        (:`then_1`
          (return true))))
    (:`Is Not Valid`
      (return false))))

(fn `UserConstructionScript`
  (set `MotionControllerComponent.MotionSource` (`|GetEnumeratorName` (`self.E_Hand`)) (`self.MotionController`)))