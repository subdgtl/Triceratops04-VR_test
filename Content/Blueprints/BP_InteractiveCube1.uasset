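; BP_InteractiveCube1 is an interactive cube actor that starts or stops spinning when activated.
; Each Activate event flips the ShouldRotate flag, then sets the RotatingMovement component's rotation rate to a constant single-axis spin or to zero.
; The component handles the motion, so Tick, BeginPlay and overlap events stay disabled and the construction script only calls its parent.
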(event `self.Activate`
  (set `self.bShouldRotate` (not (`self.bShouldRotate`)))
  (set `RotatingMovementComponent.RotationRate` (select `bool` (`self.bShouldRotate`) :`true` (struct :`Yaw` 180.0) :!type "Rotator Structure") (`self.RotatingMovement`)))

(fn `UserConstructionScript`
  (`parent.UserConstructionScript`))