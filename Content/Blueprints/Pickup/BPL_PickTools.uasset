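; BPL_PickTools is a Blueprint helper for pickup logic that finds the pickable actor nearest to a given component.
; GetActorNearComponent loops over the component's overlapping actors and keeps those implementing BPI_Pickable.
; It compares each one's distance to the component against a running nearest distance and returns the closest match.
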(fn `GetActorNearComponent`
  (params (Component :type "PrimitiveComponent Object Reference"))
  (returns (NearestActor :type "Actor Object Reference"))
  (locals (NearestOverlappingActor :type "Actor Object Reference") (NearestOverlapDistance :type "Float (double-precision)" :default 0.0))
  (for _array_element (`PrimitiveComponent.GetOverlappingActors` Component "/Script/Engine.Actor")
    (if (`KismetSystemLibrary.DoesImplementInterface` _array_element "/Game/Blueprints/Pickup/BPI_Pickable.BPI_Pickable_C")
      (bind _returnvalue (`KismetMathLibrary.VSize` (- (`Actor.K2_GetActorLocation` _array_element) (`SceneComponent.K2_GetComponentLocation` Component))))
      (if (< _returnvalue (`local.NearestOverlapDistance`))
        (`|ExecutionSequence`
          (:`then_0`
            (set `local.NearestOverlappingActor` _array_element))
          (:`then_1`
            (set `local.NearestOverlapDistance` _returnvalue))))))
  (return (`local.NearestOverlappingActor`)))