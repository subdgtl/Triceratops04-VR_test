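; BP_SnapSlot is a placement slot that previews where a BP_SnapObject will snap.
; When a snap object enters the box and none is tracked, the slot copies its mesh and scale and applies a ghost material to every slot.
; The preview clears when that object leaves, while attach and detach events toggle the in-use flag and ghost visibility.
; The construction script sizes the box from a configurable extent.
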(event `AttachToSlot`
  (set `self.SlotInUse` true)
  (`SceneComponent.SetVisibility` (`self.StaticMesh`) false false))

(event `DetachFromSlot`
  (set `self.SlotInUse` false)
  (`SceneComponent.SetVisibility` (`self.StaticMesh`) true false))

(event `self.Box.OnComponentBeginOverlap`
  (params (OverlappedComponent :type "PrimitiveComponent Object Reference") (OtherActor :type "Actor Object Reference") (OtherComp :type "PrimitiveComponent Object Reference") (OtherBodyIndex :type Integer) (bFromSweep :type Boolean) (SweepResult :type "HitResult Structure (by ref)"))
  ;[0 0 0] Show ghost mesh on overlap
  (bind _asbp_snap_object (cast `/Game/Blueprints/Pickup/BP_SnapObject` OtherActor))
  (`/Engine/EditorBlueprintResources/StandardMacros.IsValid` (`self.SnapObject`)
    (:`Is Not Valid`
      (bind _output_get (set `self.SnapObject` _asbp_snap_object))
      (bind _mesh (`/Game/Blueprints/Pickup/BP_SnapObject.Mesh` _output_get))
      (`StaticMeshComponent.SetStaticMesh` (`self.StaticMesh`) (`StaticMeshComponent.StaticMesh` _mesh))
      (`SceneComponent.SetWorldScale3D` (`self.StaticMesh`) (`SceneComponent.K2_GetComponentScale` _mesh))
      (`SceneComponent.SetVisibility` (`self.StaticMesh`) true false)
      (for _index (range (`PrimitiveComponent.GetNumMaterials` (`self.StaticMesh`)))
        (`PrimitiveComponent.SetMaterial` (`self.StaticMesh`) _index (`self.GhostMaterial`))))))

(event `self.Box.OnComponentEndOverlap`
  (params (OverlappedComponent :type "PrimitiveComponent Object Reference") (OtherActor :type "Actor Object Reference") (OtherComp :type "PrimitiveComponent Object Reference") (OtherBodyIndex :type Integer))
  ;[0 0 0] On end overlap with a snap object, if the object is the same one as the one that lastly entered stop showing the ghost mesh
  (bind _asbp_snap_object (cast `/Game/Blueprints/Pickup/BP_SnapObject` OtherActor))
  (if (== _asbp_snap_object (`self.SnapObject`))
    (`StaticMeshComponent.SetStaticMesh` (`self.StaticMesh`) null)
    (set `self.SnapObject` null)))

(fn `UserConstructionScript`
  (`BoxComponent.SetBoxExtent` (`self.Box`) (`self.SlotBoxSize`) true))