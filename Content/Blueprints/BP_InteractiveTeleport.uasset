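; BP_InteractiveTeleport is a teleport point that moves the VR player to its own location when activated.
; On BeginPlay it runs the parent logic, then casts player pawn 0 to BP_PlayerVrBase and caches it as Player.
; Its Activate event teleports that pawn to slightly above the actor's origin, keeping the pawn's current rotation.
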(event `self.ReceiveBeginPlay`
  (`parent.ReceiveBeginPlay`)
  (bind _asbp_player_vr_base (cast `/Game/Blueprints/BP_PlayerVrBase` (`GameplayStatics.GetPlayerPawn` 0)))
  (set `self.Player` _asbp_player_vr_base))

(event `self.Activate`
  (bind _player (`self.Player`))
  (`self.K2_TeleportTo` _player (+ (`self.K2_GetActorLocation`) (0.0 0.0 50.0)) (`self.K2_GetActorRotation` _player)))

(fn `UserConstructionScript`
  (`parent.UserConstructionScript`))