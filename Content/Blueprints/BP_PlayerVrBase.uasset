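; Base VR player that spawns left and right motion controllers on BeginPlay, attaches them to the camera root, and selects interactive objects by gaze.
; Each tick a camera line trace looks for a BP_InteractiveBase; a new target starts a dwell timer and spawns a BP_Timer actor above the hit point if none exists.
; When the timer elapses it activates the object and destroys the indicator; looking away cancels both.
; Mouse axes provide temporary debug head rotation, and an untimed BasicGaze variant is unused.
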(event `self.ReceiveBeginPlay`
  (bind _returnvalue (`KismetMathLibrary.MakeTransform` (0.0 0.0 0.0)))
  (bind _cameraroot (`self.CameraRoot`))
  (`|ExecutionSequence`
    (:`then_0`
      (bind _returnvalue_2 (`|SpawnActorFromClass` "/Game/Blueprints/BP_Motioncontroller.BP_Motioncontroller_C" _returnvalue "AlwaysSpawn" "OverrideRootScale" self "Left" null))
      (set `self.BP_MotionControllerL` _returnvalue_2)
      (`self.K2_AttachToComponent` _returnvalue_2 _cameraroot "None" "SnapToTarget" "SnapToTarget" "KeepRelative" true))
    (:`then_1`
      (bind _returnvalue_3 (`|SpawnActorFromClass` "/Game/Blueprints/BP_Motioncontroller.BP_Motioncontroller_C" _returnvalue "AlwaysSpawn" "OverrideRootScale" self "Right" null))
      (set `self.BP_MotionControllerR` _returnvalue_3)
      (`self.K2_AttachToComponent` _returnvalue_3 _cameraroot "None" "SnapToTarget" "SnapToTarget" "KeepRelative" true))))

(event `self.ReceiveTick`
  (params (DeltaSeconds :type "Float (single-precision)"))
  (`self.TimedBasicGaze`))

(event `InputAxisKey|MouseX`
  (params (AxisValue :type "Float (single-precision)"))
  ;[1 1 1] Temporary/debug mouse Head movement override
  (`self.AddControllerYawInput` (* (* AxisValue (`GameplayStatics.GetWorldDeltaSeconds`)) (`self.Head Move Speed`))))

(event `InputAxisKey|MouseY`
  (params (AxisValue :type "Float (single-precision)"))
  ;[1 1 1] Temporary/debug mouse Head movement override
  (`self.AddControllerPitchInput` (* (* AxisValue (`GameplayStatics.GetWorldDeltaSeconds`)) (* (`self.Head Move Speed`) -1.0))))

(fn `BasicGaze`
  (bind (_bblockinghit _binitialoverlap _time _distance _location _impactpoint _normal _impactnormal _physmat _hitactor) (`GameplayStatics.BreakHitResult` (`self.LineTrace`)))
  (if _bblockinghit
    (bind _asbp_interactive_base (cast `/Game/Blueprints/BP_InteractiveBase` _hitactor)
      (:`then`
        (set `self.Interactive Object` _asbp_interactive_base)
        (if (not (== (`self.Interactive Object`) (`self.Focused Object`)))
          (set `self.Focused Object` (`self.Interactive Object`))
          (`self.Interact`)))
      (:`CastFailed`
        (set `self.Interactive Object` null :!label _label)
        (set `self.Focused Object` null)))
    (else
      (goto _label))))

(fn `Interact`
  (bind _interactive_object (`self.Interactive Object`))
  (bind _timerref (`self.TimerRef`))
  (`/Engine/EditorBlueprintResources/StandardMacros.IsValid` _interactive_object
    (:`Is Valid`
      (`/Game/Blueprints/BP_InteractiveBase.Activate` _interactive_object)
      (`/Engine/EditorBlueprintResources/StandardMacros.IsValid` _timerref
        (:`Is Valid`
          (`self.K2_DestroyActor` _timerref))))))

(fn `LineTrace`
  (returns (OutHit :type "HitResult Structure"))
  (bind _camera (`self.Camera`))
  (bind _returnvalue (`SceneComponent.K2_GetComponentLocation` _camera))
  (bind _outhit (`KismetSystemLibrary.LineTraceSingle` _returnvalue (+ _returnvalue (* (`KismetMathLibrary.GetForwardVector` (`SceneComponent.K2_GetComponentRotation` _camera)) 2500.0)) "TraceTypeQuery1"))
  (return _outhit))

(fn `TimedBasicGaze`
  (bind _timerref (`self.TimerRef`))
  (bind (_bblockinghit _binitialoverlap _time _distance _location _impactpoint _normal _impactnormal _physmat _hitactor) (`GameplayStatics.BreakHitResult` (`self.LineTrace`)))
  (if _bblockinghit
    (bind _asbp_interactive_base (cast `/Game/Blueprints/BP_InteractiveBase` _hitactor)
      (:`then`
        (set `self.Interactive Object` _asbp_interactive_base)
        (if (not (== (`self.Interactive Object`) (`self.Focused Object`)))
          (set `self.Focused Object` (`self.Interactive Object`))
          (`KismetSystemLibrary.K2_ClearAndInvalidateTimerHandle` (`self.FocusTimer`))
          (bind _returnvalue (`KismetSystemLibrary.K2_SetTimer` null "Interact" (`self.TimerLenght`)))
          (set `self.FocusTimer` _returnvalue)
          (`/Engine/EditorBlueprintResources/StandardMacros.IsValid` (`self.TimerRef`)
            (:`Is Not Valid`
              (bind _returnvalue_2 (`|SpawnActorFromClass` "/Game/Blueprints/BP_Timer.BP_Timer_C" (`KismetMathLibrary.MakeTransform` (+ _impactpoint (0.0 0.0 150.0))) "Undefined" "OverrideRootScale" null null))
              (set `self.TimerRef` _returnvalue_2)))))
      (:`CastFailed`
        (set `self.Interactive Object` null :!label _label)
        (set `self.Focused Object` null)
        (`KismetSystemLibrary.K2_ClearAndInvalidateTimerHandle` (`self.FocusTimer`))
        (`/Engine/EditorBlueprintResources/StandardMacros.IsValid` _timerref
          (:`Is Valid`
            (`self.K2_DestroyActor` _timerref)))))
    (else
      (goto _label))))

(fn `UserConstructionScript`)